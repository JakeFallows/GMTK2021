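; SoulController is a player controller Blueprint that handles the player's death sequence.
; Its OnDeath event unpossesses the pawn, starts a held camera fade-out and shows a DeathScreen widget.
; After a short delay it removes the widget and calls RestartGame on SoulGameMode, printing a debug string if that cast fails.
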(event `/Game/Blueprints/Interfaces/Damageable.OnDeath`
  (`self.UnPossess`)
  (`PlayerCameraManager.StartCameraFade` :`self` (`self.PlayerCameraManager`) :`ToAlpha` 1.0 :`Duration` 1.0 :`bHoldWhenFinished` true)
  (bind _returnvalue (`|CreateWidget` "/Game/UI/DeathScreen.DeathScreen_C" self))
  (`UserWidget.AddToViewport` _returnvalue 0)
  (`KismetSystemLibrary.Delay` 2.0)
  (`Widget.RemoveFromParent` _returnvalue)
  (bind _assoul_game_mode (cast `/Game/Blueprints/SoulGameMode` (`GameplayStatics.GetGameMode`))
    (:`then`
      (`GameMode.RestartGame` _assoul_game_mode))
    (:`CastFailed`
      (`KismetSystemLibrary.PrintString` "OOF"))))

(fn `UserConstructionScript`)