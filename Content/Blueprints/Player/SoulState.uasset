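; SoulState holds the player soul's state: health, adopted pets and fire rate.
; Adopting a pet marks it adopted, adds its health to both max and current health, and notifies it.
; Damage reduces current health and triggers OnDeath on the SoulController at zero or below.
; It also creates the HUD on BeginPlay, shows and clears a SoulJoined widget, and derives fire delay inversely from fire rate.
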(event `self.ReceiveBeginPlay`
  (`self.Add HUD`))

(event `/Game/Blueprints/Interfaces/Damageable.TakeDamage`
  (params (damage :type "Float (single-precision)"))
  (bind _output_get (set `self.currentHealth` (- (`self.currentHealth`) damage)))
  (`KismetSystemLibrary.PrintString` (`KismetStringLibrary.Conv_DoubleToString` _output_get))
  (if (<= (`self.currentHealth`) 0.0)
    (bind _assoul_controller (cast `/Game/Blueprints/Player/SoulController` (`GameplayStatics.GetPlayerController` 0)))
    (`/Game/Blueprints/Interfaces/Damageable.OnDeath` _assoul_controller)))

(fn `Add HUD`
  (bind _returnvalue (`|CreateWidget` "/Game/UI/HUD.HUD_C"))
  (bind _output_get (set `self.HUD` _returnvalue))
  (`UserWidget.AddToViewport` _output_get 0))

(fn `Adoption`
  (params (newPet :type "/Game/Blueprints/Allies/BasePet Object Reference"))
  (bind _health (`/Game/Blueprints/Allies/BasePet.health` newPet))
  (`KismetArrayLibrary.Array_AddUnique` (`self.pets`) newPet)
  (set `/Game/Blueprints/Allies/BasePet.adopted` true newPet)
  (set `self.maxHealth` (+ (`self.maxHealth`) _health))
  (set `self.currentHealth` (+ (`self.currentHealth`) _health))
  (message `/Game/Blueprints/Interfaces/Adoptable.getAdopted` newPet self))

(fn `calculateFireDelay`
  (returns (delay :type "Float (double-precision)"))
  (return (/ 3.0 (`self.fireRate`))))

(fn `Clear Soul Joined`
  (`Widget.RemoveFromParent` (`self.SoulJoined`)))

(fn `Soul Joined`
  (bind _assoul_controller (cast `/Game/Blueprints/Player/SoulController` (`GameplayStatics.GetPlayerController` 0)))
  (bind _returnvalue (`|CreateWidget` "/Game/UI/SoulJoined.SoulJoined_C" _assoul_controller))
  (bind _output_get (set `self.SoulJoined` _returnvalue))
  (`UserWidget.AddToViewport` _output_get 0))

(fn `UserConstructionScript`)