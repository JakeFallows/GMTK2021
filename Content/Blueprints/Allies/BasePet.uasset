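; Base Blueprint for an ally pet that follows the player once it has been adopted.
; While Adopted is set, every Tick casts player pawn 0 to SoulPawn and issues AIMoveTo with that pawn as the target actor.
; A RandomizeHeight helper shifts a given static mesh vertically by a random offset of up to 75 units up or down, but nothing in this graph calls it.
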(event `self.ReceiveTick`
  (params (DeltaSeconds :type "Float (single-precision)"))
  (if (`self.adopted`)
    (bind _assoul_pawn (cast `/Game/Blueprints/Player/SoulPawn` (`GameplayStatics.GetPlayerPawn` 0)))
    (`|AIMoveTo` self (0.0 0.0 50.0) _assoul_pawn)))

(fn `randomizeHeight`
  (params (staticMesh :type "StaticMeshComponent Object Reference"))
  (`SceneComponent.K2_SetWorldLocation` staticMesh (`KismetMathLibrary.MakeVector` (.x (`SceneComponent.K2_GetComponentLocation` staticMesh)) (.y (`SceneComponent.K2_GetComponentLocation` staticMesh)) (+ (.z (`SceneComponent.K2_GetComponentLocation` staticMesh)) (- (* (`KismetMathLibrary.RandomFloat`) 150.0) 75.0))) false false))

(fn `UserConstructionScript`)