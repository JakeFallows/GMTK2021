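; Adoptable ally pet that acts as a "Fire Rate Up" upgrade.
; On BeginPlay it sets its description and randomizes its mesh height.
; GetAdopted raises the fire rate on the passed State by one step, up to a cap.
; Overlapping a SoulPawn adds a Niagara effect to that pawn, then destroys the pet after a short delay.
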(event `self.ReceiveBeginPlay`
  (set `self.description` "Fire Rate Up")
  (`self.randomizeHeight` (`self.StaticMesh`)))

(event `/Game/Blueprints/Interfaces/Adoptable.getAdopted`
  (params (state :type "/Game/Blueprints/Player/SoulState Object Reference"))
  (set `/Game/Blueprints/Player/SoulState.fireRate` (`KismetMathLibrary.FMin` (+ (`/Game/Blueprints/Player/SoulState.fireRate` state) 1.0) 10.0) state))

(event `self.ReceiveActorBeginOverlap`
  (params (OtherActor :type "Actor Object Reference"))
  (bind _assoul_pawn (cast `/Game/Blueprints/Player/SoulPawn` OtherActor))
  (`AddComponent|NODE_AddNiagaraComponent-2` :`self` _assoul_pawn)
  (`KismetSystemLibrary.Delay` 0.5)
  (`self.K2_DestroyActor`))

(fn `UserConstructionScript`
  (`parent.UserConstructionScript`))