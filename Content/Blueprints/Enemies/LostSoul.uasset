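; Lost Soul enemy that chases pawns it sees and fires projectiles at the player.
; PawnSensing or taking damage starts an AI move toward the last sensed pawn, setting a brief InSight flag.
; Tick stops it in range and, while InSight, spawns a delayed LostSoulProjectile aimed at the player, then moves to a random nearby navigable point before resuming the chase.
; Damage reduces Health and destroys it at zero.
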(event `self.PawnSensing.OnSeePawn`
  (params (Pawn :type "Pawn Object Reference"))
  (if (not (`self.firedRecently`))
    (`|AIMoveTo` self (0.0 0.0 0.0) Pawn 70.0 :!label _label
      (:`then`
        (set `self.inSight` true))
      (:`OnSuccess`
        (`KismetSystemLibrary.Delay` 0.2 :!label _label_2)
        (set `self.inSight` false))
      (:`OnFail`
        (goto _label_2)))))

(event `self.ReceiveTick`
  (params (DeltaSeconds :type "Float (single-precision)"))
  (bind _isinrange (`self.isInAttackRange`))
  (if (and _isinrange (not (`self.firedRecently`)))
    (`MovementComponent.StopMovementImmediately` (`self.CharacterMovement`)))
  (if (and (`self.inSight`) _isinrange)
    (`KismetSystemLibrary.Delay` 0.5)
    (bind _returnvalue (`self.toPlayerTransform`))
    (`|SpawnActorFromClass` "/Game/Blueprints/Projectiles/LostSoulProjectile.LostSoulProjectile_C" _returnvalue "AdjustIfPossibleButDontSpawnIfColliding" "OverrideRootScale" null null)
    (set `self.firedRecently` true)
    (bind _randomlocation (`NavigationSystemV1.K2_GetRandomLocationInNavigableRadius` (`SceneComponent.K2_GetComponentLocation` (`self.Mesh`)) 200.0 null "/Script/AIModule.NavFilter_AIControllerDefault"))
    (`|AIMoveTo` self _randomlocation null
      (:`OnSuccess`
        _)
      (:`OnFail`
        _))
    (set `self.firedRecently` false)
    (`|AIMoveTo` self (0.0 0.0 0.0) (`GameplayStatics.GetPlayerPawn` 0))))

(event `/Game/Blueprints/Interfaces/Damageable.TakeDamage`
  (params (damage :type "Float (single-precision)"))
  (`|ExecutionSequence`
    (:`then_0`
      (bind _output_get (set `self.health` (- (`self.health`) damage)))
      (if (<= _output_get 0.0)
        (`self.K2_DestroyActor`)))
    (:`then_1`
      (goto _label))))

(event `self.ReceiveBeginPlay`
  (`SkeletalMeshComponent.PlayAnimation` (`self.Mesh`) "/Game/Skeletal_Meshes/Eye_Bat_Demon_WAnim_Anim_Armature_Idle.Eye_Bat_Demon_WAnim_Anim_Armature_Idle" true))

(fn `isInAttackRange`
  (returns (isInRange :type Boolean) (distance :type "Float (double-precision)"))
  (bind _returnvalue (`self.GetDistanceTo` self (`GameplayStatics.GetPlayerPawn` 0)))
  (return (<= _returnvalue 500.0) _returnvalue))

(fn `toPlayerTransform`
  (returns (ReturnValue :type "Transform Structure"))
  (bind _returnvalue (`SceneComponent.K2_GetComponentLocation` (`self.Mesh`)))
  (return (`KismetMathLibrary.MakeTransform` _returnvalue (`KismetMathLibrary.Conv_VectorToRotator` (`KismetMathLibrary.GetDirectionUnitVector` _returnvalue (`self.K2_GetActorLocation` (`GameplayStatics.GetPlayerPawn` 0)))))))

(fn `UserConstructionScript`)